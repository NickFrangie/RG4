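; Base player character with camera-relative movement, hold-to-sprint, multi-jump, dash and grappling hook.
; Dash pops up, launches forward and briefly suspends gravity, recharging when grounded.
; Grapple filters BP_GrapplePoint actors by screen position, picks the nearest, switches to Flying and shows the cable.
; Tick pulls toward that point with strafe steering until within range, while button release restores Falling and hides the cable.
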(event EventBeginPlay
  (Variables|Default|SetDefaii;t%20Walk%20Speed (Variables|/Script/Engine.CharacterMovementComponent|GetMaxWalkSpeed (Variables|Character|GetCharacterMovement))))

(event Collision|EventActorBeginOverlap
  (params (OtherActor :type Actor%20Object%20Reference)))

(event EventTick
  (params (DeltaSeconds :type Float%20%28single-precision%29)))

(event EventTick
  (params (DeltaSeconds :type Float%20%28single-precision%29))
  ;[0 0 0] Check for dash reset
  (if (AI|Components|NavMovement|IsMovingonGround (Variables|Character|GetCharacterMovement))
    (Variables|Default|SetHasDash true))
  ;[0 0 0] Apply Grapple Force
  (if (Variables|Default|GetIsGrapple)
    (Physics|AddForce (Variables|Character|GetCharacterMovement) (* (Math|Vector|Normalize (+ (Math|Vector|GetUnitDirection(Vector) (Transformation|GetActorLocation) (Variables|Default|GetGrapple%20Point%20Location)) (* (Input|AxisValues|GetMoveRight) (Transformation|GetActorRightVector) 0.5))) 3e+05))
    (Variables|/Script/CableComponent.CableComponent|SetEndLocation (Variables|Default|GetCable) (Math|Transform|InverseTransformLocation (Transformation|GetActorTransform) (Variables|Default|GetGrapple%20Point%20Location)))
    (if (<= (Math|Vector|Distance(Vector) (Variables|Default|GetGrapple%20Point%20Location) (Transformation|GetActorLocation)) 1e+02)
      (Variables|Default|SetIsGrapple false))))

(event Input|ActionEvents|InputActionJump
  (params (Key :type Key%20Structure :default "None"))
  ;[0 0 0] Jump + Double Jumo
  (:Pressed
    (if (< (Variables|Default|GetJumpCurrentCount) (Variables|Default|GetJumpMaxCount))
      (if (AI|Components|NavMovement|IsFalling (Variables|Character|GetCharacterMovement))
        (Animation|PlayAnimMontage 0 1.0 "None")
        (Character|Jump)
        (else
          (Character|Jump)))))
  (:Released
    (Character|StopJumping)))

(event Input|ActionEvents|InputActionSprint
  (params (Key :type Key%20Structure :default "None"))
  ;[0 0 0] Sprint Toggle Logic
  (:Pressed
    (Variables|/Script/Engine.CharacterMovementComponent|SetMaxWalkSpeed (Variables|Character|GetCharacterMovement) (* 3.0 (Variables|Default|GetDefaii;t%20Walk%20Speed))))
  (:Released
    (Variables|/Script/Engine.CharacterMovementComponent|SetMaxWalkSpeed (Variables|Character|GetCharacterMovement) (Variables|Default|GetDefaii;t%20Walk%20Speed))))

(event Input|ActionEvents|InputActionGrapple
  (params (Key :type Key%20Structure :default "None"))
  (bind _returnvalue (Viewport|GetViewportSize))
  ;[0 0 0] Find Best GrapplePoint on press Grapple button
  (:Pressed
    (bind _outactors (Actor|GetAllActorsOfClass "/Game/Blueprints/BP_GrapplePoint.BP_GrapplePoint_C"))
    ;;[0 0 0] Remove GrapplePoints not on screen
    (for _array_element _outactors
      (if (not (Math|Boolean|ANDBoolean (> (.x (.ScreenLocation (Class|PlayerController|ProjectWorldLocationtoScreen (Game|GetPlayerController 0) (Transformation|GetActorLocation _array_element) true))) 0.0) (> (.y (.ScreenLocation (Class|PlayerController|ProjectWorldLocationtoScreen (Game|GetPlayerController 0) (Transformation|GetActorLocation _array_element) true))) 0.0) (< (.x (.ScreenLocation (Class|PlayerController|ProjectWorldLocationtoScreen (Game|GetPlayerController 0) (Transformation|GetActorLocation _array_element) true))) (.x _returnvalue)) (< (.y (.ScreenLocation (Class|PlayerController|ProjectWorldLocationtoScreen (Game|GetPlayerController 0) (Transformation|GetActorLocation _array_element) true))) (.y _returnvalue))))
        (Utilities|Array|RemoveItem _outactors _array_element)))
    (Development|PrintString (Utilities|String|ToString(Integer) (Utilities|Array|Length _outactors)))
    (Variables|Default|SetGrapple%20Point%20Location (Transformation|GetActorLocation (.ReturnValue (Actor|FindNearestActor (Transformation|GetWorldLocation (Variables|Collision|GetCapsuleComponent)) _outactors))))
    (Variables|Default|SetIsGrapple true)
    (Pawn|Components|CharacterMovement|SetMovementMode (Variables|Character|GetCharacterMovement) "MOVE_Flying" 0)
    (Rendering|SetVisibility (Variables|Default|GetCable) true false))
  (:Released
    (Variables|Default|SetIsGrapple false)
    (Pawn|Components|CharacterMovement|SetMovementMode (Variables|Character|GetCharacterMovement) "MOVE_Falling" 0)
    (Rendering|SetVisibility (Variables|Default|GetCable) false false)))

(event Input|ActionEvents|InputActionDash
  (params (Key :type Key%20Structure :default "None"))
  (:Pressed
    (if (Variables|Default|GetHasDash)
      (Development|PrintString "Dashed")
      ;[0 0 0] Dash (Ground and Mid-air)
      (Variables|Default|SetHasDash false)
      (Utilities|FlowControl|DoOnce false :!label _label
        (:Completed
          (Character|LaunchCharacter "0.000000,0.000000,50.000000" false false)
          (Utilities|FlowControl|Delay 0.01)
          (Character|LaunchCharacter (* (Math|Vector|GetForwardVector (Transformation|GetActorRotation)) 3e+03) true true)
          (Animation|PlayAnimMontage 0 1.0 "None")
          (Variables|/Script/Engine.CharacterMovementComponent|SetGravityScale (Variables|Character|GetCharacterMovement) 0.0)
          (Utilities|FlowControl|Delay 0.25)
          (Variables|/Script/Engine.CharacterMovementComponent|SetGravityScale (Variables|Character|GetCharacterMovement) 5.0)
          (goto _label Reset))))))

(event Input|AxisEvents|InputAxisMoveForward
  (params (AxisValue :type Float%20%28single-precision%29))
  (bind _returnvalue (Pawn|GetControlRotation :!class /Script/Engine.Pawn))
  (bind (_roll _pitch _yaw) (Math|Rotator|BreakRotator _returnvalue))
  ;[0 0 0 1 30] Directional Movement Logic
  (Pawn|Input|AddMovementInput (Math|Vector|GetForwardVector (Math|Rotator|MakeRotator 0.0 _pitch _yaw)) AxisValue false))

(event Input|AxisEvents|InputAxisMoveRight
  (params (AxisValue :type Float%20%28single-precision%29))
  (bind _returnvalue (Pawn|GetControlRotation :!class /Script/Engine.Pawn))
  (bind (_roll _pitch _yaw) (Math|Rotator|BreakRotator _returnvalue))
  ;[0 0 0 1 30] Directional Movement Logic
  (Pawn|Input|AddMovementInput (Math|Vector|GetRightVector (Math|Rotator|MakeRotator 0.0 _pitch _yaw)) AxisValue false))

(event Input|AxisEvents|InputAxisTurn
  (params (AxisValue :type Float%20%28single-precision%29))
  ;[0 0 0] Mouse Look Logic
  (Pawn|Input|AddControllerYawInput AxisValue))

(event Input|AxisEvents|InputAxisLookUp
  (params (AxisValue :type Float%20%28single-precision%29))
  ;[0 0 0] Mouse Look Logic
  (Pawn|Input|AddControllerPitchInput AxisValue))

(fn ConstructionScript)