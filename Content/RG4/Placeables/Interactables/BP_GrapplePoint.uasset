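; BP_GrapplePoint is a placeable grapple point that can be highlighted as the current target.
; SetTarget clears the highlight on every grapple point in the level, then sets its own Target component's custom depth stencil to mark it exclusively.
; The construction script creates a dynamic outline material on Target.
; Logic to scale outline width inversely with distance to BP_RobotPawn is disconnected, so Tick does nothing.
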(event EventBeginPlay)

(event Collision|EventActorBeginOverlap
  (params (OtherActor :type Actor%20Object%20Reference)))

(event EventTick
  (params (DeltaSeconds :type Float%20%28single-precision%29)))

(fn ConstructionScript
  (bind _returnvalue (Rendering|Material|CreateDynamicMaterialInstance (Variables|Default|GetTarget) 1 "/Game/Developers/AlexMarrinan/TargetOutline.TargetOutline" "width" :!class /Script/Engine.PrimitiveComponent))
  (Variables|Default|SetTargetOutline _returnvalue))

(fn SetTarget
  (bind _outactors (Actor|GetAllActorsOfClass "BP_GrapplePoint_C"))
  (for _array_element _outactors
    (CallFunction|HideTarget _array_element))
  (Rendering|SetCustomDepthStencilValue (Variables|Default|GetTarget) 2))

(fn HideTarget
  (Rendering|SetCustomDepthStencilValue (Variables|Default|GetTarget) 0))