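; BP_Door is a placeable door that opens once all of its linked interactables are activated.
; On BeginPlay it binds to the interaction event of each key in its Interactables map, then records each reported activation state in that map.
; When no value is false, OpenDoor plays the hatch animation once without looping and disables its collision.
; It has no closing logic.
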(event Custom|Interactable%20Interaction%20Event
  (params (interactable :type BP%20Interactable%20Object%20Reference) (activated :type Boolean))
  (bind _interactables (Variables|Default|GetInteractables))
  (Utilities|Map|Add _interactables interactable activated)
  (bind _values (Utilities|Map|Values _interactables))
  (if (not (Utilities|Array|ContainsItem _values false))
    (CallFunction|OpenDoor)))

(event EventBeginPlay
  (bind _keys (Utilities|Map|Keys (Variables|Default|GetInteractables)))
  (for _array_element _keys
    (EventDispatchers|BindEventtoInteractionEvent _array_element (delegate Custom|Interactable%20Interaction%20Event))))

(event Collision|EventActorBeginOverlap
  (params (OtherActor :type Actor%20Object%20Reference)))

(event EventTick
  (params (DeltaSeconds :type Float%20%28single-precision%29)))

(fn ConstructionScript)

(fn OpenDoor
  (bind _ob_hatchdoor (Variables|Default|GetOB_HatchDoor))
  (Audio|Components|Audio|Play _ob_hatchdoor false)
  (Collision|SetCollisionEnabled _ob_hatchdoor "NoCollision"))