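; BP_Lever is a placeable lever interactable that is pulled by overlap.
; When an overlapping actor has a BP_Interactor component whose CanInteract returns true, it plays the lever animation without looping and fires InteractionEvent with itself as activated.
; An IsPressed latch makes it one-shot, since nothing in this Blueprint resets it.
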(event OnComponentBeginOverlap(Collider)
  (params (OverlappedComponent :type Primitive%20Component%20Object%20Reference) (OtherActor :type Actor%20Object%20Reference) (OtherComp :type Primitive%20Component%20Object%20Reference) (OtherBodyIndex :type Integer) (bFromSweep :type Boolean) (SweepResult :type Hit%20Result%20Structure%20%28by%20ref%29))
  (bind _returnvalue (Actor|GetComponentbyClass OtherActor "/Game/RG4/Core/Interactables/Component/BP_Interactor.BP_Interactor_C"))
  (Utilities|IsValid _returnvalue
    (:Is%20Valid
      (bind _caninteract (Default|CanInteract _returnvalue))
      (if _caninteract
        (if (not (Variables|Default|GetisPressed))
          (Variables|Default|SetisPressed true)
          (Audio|Components|Audio|Play (Variables|Default|GetOB_Lever_Animated_01) false)
          (Default|CallInteractionEvent self true))))))

(event EventBeginPlay)

(event Collision|EventActorBeginOverlap
  (params (OtherActor :type Actor%20Object%20Reference)))

(event EventTick
  (params (DeltaSeconds :type Float%20%28single-precision%29)))

(fn ConstructionScript)