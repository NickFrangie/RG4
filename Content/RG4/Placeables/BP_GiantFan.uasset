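; A placeable giant fan that pushes the robot pawn with wind while it stands inside the fan's trigger.
; WindTrigger overlap events set a PlayerInFan flag when a BP_RobotPawn enters or leaves.
; Each Tick while flagged, it looks up the robot pawn by class and calls ApplyFanForce along the fan's up vector, scaled by WindForce.
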(event OnComponentBeginOverlap(WindTrigger)
  (params (OverlappedComponent :type Primitive%20Component%20Object%20Reference) (OtherActor :type Actor%20Object%20Reference) (OtherComp :type Primitive%20Component%20Object%20Reference) (OtherBodyIndex :type Integer) (bFromSweep :type Boolean) (SweepResult :type Hit%20Result%20Structure%20%28by%20ref%29))
  (Development|PrintString "entered fan" true true "(R=0.000000,G=0.660000,B=1.000000,A=1.000000)" 2.0 "fanstatus")
  (if (== (Utilities|GetClass OtherActor) "/Game/RG4/Core/BP_RobotPawn.BP_RobotPawn_C")
    (Variables|Default|SetPlayerInFan true)))

(event OnComponentEndOverlap(WindTrigger)
  (params (OverlappedComponent :type Primitive%20Component%20Object%20Reference) (OtherActor :type Actor%20Object%20Reference) (OtherComp :type Primitive%20Component%20Object%20Reference) (OtherBodyIndex :type Integer))
  (Development|PrintString "entered fan" true true "(R=0.000000,G=0.660000,B=1.000000,A=1.000000)" 2.0 "fanstatus")
  (if (== (Utilities|GetClass OtherActor) "/Game/RG4/Core/BP_RobotPawn.BP_RobotPawn_C")
    (Variables|Default|SetPlayerInFan false)))

(event EventBeginPlay)

(event Collision|EventActorBeginOverlap
  (params (OtherActor :type Actor%20Object%20Reference)))

(event EventTick
  (params (DeltaSeconds :type Float%20%28single-precision%29))
  (if (Variables|Default|GetPlayerInFan)
    (bind _returnvalue (Actor|GetActorOfClass "/Game/RG4/Core/BP_RobotPawn.BP_RobotPawn_C"))
    (Default|ApplyFanForce _returnvalue (* (Math|Vector|GetUpVector (Transformation|GetActorRotation)) (Variables|Default|GetWind%20Force)))))

(fn ConstructionScript)