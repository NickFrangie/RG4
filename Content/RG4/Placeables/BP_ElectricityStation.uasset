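; Placeable electricity station that acts as a hazard for the player, applying a full health bar's worth of damage on contact.
; On BeginPlay it caches the player pawn as a BP_ThirdPersonCharacter.
; When that player overlaps the Box, it calls ApplyDamage with the negated MaxHealth from the player's BP_HealthComponent, so the damage value passed is negative.
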(event OnComponentBeginOverlap(Box)
  (params (OverlappedComponent :type Primitive%20Component%20Object%20Reference) (OtherActor :type Actor%20Object%20Reference) (OtherComp :type Primitive%20Component%20Object%20Reference) (OtherBodyIndex :type Integer) (bFromSweep :type Boolean) (SweepResult :type Hit%20Result%20Structure%20%28by%20ref%29))
  (bind _playerref (Variables|Default|GetPlayerRef))
  (if (== OtherActor _playerref)
    (Game|Damage|ApplyDamage (Variables|Default|GetPlayerRef) (Math|Conversions|ToFloat(Integer) (* -1 (Variables|/Game/RG4/Core/EnergySystem/BP_HealthComponent.BP_HealthComponent_C|GetMaxHealth (Actor|GetComponentbyClass _playerref "/Game/RG4/Core/EnergySystem/BP_HealthComponent.BP_HealthComponent_C")))) 0 0)))

(event EventBeginPlay
  (bind _asbp_third_person_character (Utilities|Casting|CastToBP_ThirdPersonCharacter (Game|Player|GetPlayerPawn 0)))
  (Variables|Default|SetPlayerRef _asbp_third_person_character))

(fn ConstructionScript)