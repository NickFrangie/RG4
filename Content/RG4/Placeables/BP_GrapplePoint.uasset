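; Placeable grapple point that can be highlighted as the current target.
; SetTarget clears the highlight on every grapple point, then sets this one's Custom Depth stencil to mark it.
; Construction creates a dynamic outline material on the Target component.
; Each Tick sets that material's width inversely to the distance from the first BP_RobotPawn, found with GetAllActorsOfClass every frame.
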(event EventBeginPlay)

(event Collision|EventActorBeginOverlap
  (params (OtherActor :type Actor%20Object%20Reference)))

(event EventTick
  (params (DeltaSeconds :type Float%20%28single-precision%29))
  (bind _targetoutline (Variables|Default|GetTargetOutline))
  (bind _outactors (Actor|GetAllActorsOfClass "/Game/RG4/Core/BP_RobotPawn.BP_RobotPawn_C"))
  (Rendering|Material|SetScalarParameterValue _targetoutline "width" (/ 1e+11 (Math|Vector|Distance(Vector) (Transformation|GetActorLocation (Utilities|Array|Get(acopy) _outactors)) (Transformation|GetActorLocation))) :!class /Script/Engine.MaterialInstanceDynamic)
  (Rendering|Material|GetScalarParameterValue _targetoutline "width" :!class /Script/Engine.MaterialInstanceDynamic))

(fn ConstructionScript
  (bind _returnvalue (Rendering|Material|CreateDynamicMaterialInstance (Variables|Default|GetTarget) 1 "/Game/Developers/AlexMarrinan/TargetOutline.TargetOutline" "width" :!class /Script/Engine.PrimitiveComponent))
  (Variables|Default|SetTargetOutline _returnvalue))

(fn SetTarget
  (bind _outactors (Actor|GetAllActorsOfClass "BP_GrapplePoint_C"))
  (for _array_element _outactors
    (CallFunction|HideTarget _array_element))
  (Rendering|SetCustomDepthStencilValue (Variables|Default|GetTarget) 2))

(fn HideTarget
  (Rendering|SetCustomDepthStencilValue (Variables|Default|GetTarget) 0))