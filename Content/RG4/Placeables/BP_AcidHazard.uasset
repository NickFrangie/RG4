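; BP_AcidHazard is a placeable hazard that periodically damages actors inside its box.
; Box begin overlap adds actors that have a BP_HealthComponent to ActorsToDamage.
; A looping timer started at BeginPlay applies configurable damage and damage type to every listed actor.
; End overlap calls removal only when the found index is zero or below, so actors later in the list keep taking damage after leaving.
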(event OnComponentBeginOverlap(Box)
  (params (OverlappedComponent :type Primitive%20Component%20Object%20Reference) (OtherActor :type Actor%20Object%20Reference) (OtherComp :type Primitive%20Component%20Object%20Reference) (OtherBodyIndex :type Integer) (bFromSweep :type Boolean) (SweepResult :type Hit%20Result%20Structure%20%28by%20ref%29))
  (Utilities|IsValid (Actor|GetComponentbyClass OtherActor "/Game/RG4/Core/EnergySystem/BP_HealthComponent.BP_HealthComponent_C")
    (:Is%20Valid
      (Utilities|Array|Add (Variables|Default|GetActorsToDamage) OtherActor))))

(event OnComponentEndOverlap(Box)
  (params (OverlappedComponent :type Primitive%20Component%20Object%20Reference) (OtherActor :type Actor%20Object%20Reference) (OtherComp :type Primitive%20Component%20Object%20Reference) (OtherBodyIndex :type Integer))
  (bind _actorstodamage (Variables|Default|GetActorsToDamage))
  (bind _returnvalue (Utilities|Array|FindItem _actorstodamage OtherActor))
  (if (<= _returnvalue 0)
    (Utilities|Array|RemoveIndex (Variables|Default|GetActorsToDamage) _returnvalue)))

(event Custom|DamageTake
  (for _array_element (Variables|Default|GetActorsToDamage)
    (CallFunction|DamageActor _array_element)))

(event EventBeginPlay
  (Utilities|Time|SetTimerbyEvent (delegate Custom|DamageTake) 3.0 true))

(fn ConstructionScript)

(fn DamageActor
  (params (Actor :type Actor%20Object%20Reference))
  (Game|Damage|ApplyDamage Actor (Math|Conversions|ToFloat(Integer) (Variables|Default|GetBase%20Damage)) 0 0 "/Script/Engine.DamageType"))