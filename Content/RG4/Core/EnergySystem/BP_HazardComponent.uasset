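; BP_HazardComponent is a component that lets its owning hazard damage and knock back actors that collide with it.
; OnHazardCollision passes HazardDamage to the other actor's BP_HealthComponent via OnTakeAnyDamage.
; Damage above a fixed threshold also passes the player pawn as DamagedActor so instant kills bypass invincibility, and skips knockback.
; Otherwise, including without damage or health component, a positive KnockbackForce knocks BP_RobotPawn back relative to the owner's location.
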(event EventBeginPlay)

(event EventTick
  (params (DeltaSeconds :type Float%20%28single-precision%29)))

(fn OnHazardCollision
  (params (Other :type Actor%20Object%20Reference))
  (bind _returnvalue (Actor|GetComponentbyClass Other "/Game/RG4/Core/EnergySystem/BP_HealthComponent.BP_HealthComponent_C"))
  (if (> (Variables|Default|GetHazardDamage) 0)
    ;[1 1 1] Damage
    (Utilities|IsValid _returnvalue
      (:Is%20Valid
        (if (> (Variables|Default|GetHazardDamage) 4)
          (Default|OnTakeAnyDamage _returnvalue (Game|Player|GetPlayerPawn 0) (Math|Conversions|ToFloat(Integer) (Variables|Default|GetHazardDamage)))
          (else
            (Default|OnTakeAnyDamage _returnvalue 0 (Math|Conversions|ToFloat(Integer) (Variables|Default|GetHazardDamage)))
            (if (> (Variables|Default|GetKnockbackForce) 0.0) :!label _label
              ;[1 1 1] Knockback
              (bind _asbp_robot_pawn (Utilities|Casting|CastToBP_RobotPawn Other))
              (Utilities|IsValid _asbp_robot_pawn
                (:Is%20Valid
                  (Default|ApplyDamageKnockback _asbp_robot_pawn (Transformation|GetActorLocation (Components|GetOwner)) (Variables|Default|GetKnockbackForce))))))))
      (:Is%20Not%20Valid
        (goto _label)))
    (else
      (goto _label))))