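; BP_HealthComponent is a health component that tracks its owner's health and displays it as a battery-style HUD.
; On BeginPlay it fills health, adds WBP_BatteryUI to player 0's viewport and binds to the owner's OnTakeAnyDamage.
; Damage lowers the clamped integer health, broadcasts OnHealthChange, updates the battery cell color and fires OnDeath at zero.
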(event Custom|OnTakeAnyDamage
  (params (DamagedActor :type Actor%20Object%20Reference) (Damage :type Float%20%28single-precision%29) (DamageType :type Damage%20Type%20Object%20Reference) (InstigatedBy :type Controller%20Object%20Reference) (DamageCauser :type Actor%20Object%20Reference))
  (bind _output_get (Variables|Default|SetHealth (Math|Integer|Clamp(Integer) (Math|Float|Truncate (- (Variables|Default|GetHealth) Damage)) 0 (Variables|Default|GetMaxHealth))))
  (Default|CallOnHealthChange _output_get (Variables|Default|GetMaxHealth))
  (CallFunction|SetBatteryColor)
  (if (<= (Variables|Default|GetHealth) 0)
    (Default|CallOnDeath)))

(event EventBeginPlay
  (Variables|Default|SetHealth (Variables|Default|GetMaxHealth))
  (CallFunction|CreateBatteryUI)
  (EventDispatchers|AssignOnTakeAnyDamage (Components|GetOwner) (delegate Custom|OnTakeAnyDamage)))

(fn CreateBatteryUI
  (bind _returnvalue (UserInterface|CreateWidget "/Game/RG4/Core/EnergySystem/WBP_BatteryUI.WBP_BatteryUI_C" (Game|GetPlayerController 0)))
  (bind _output_get (Variables|Default|SetBattery%20UI _returnvalue))
  (Utilities|IsValid _output_get
    (:Is%20Valid
      (UserInterface|Viewport|AddtoViewport _output_get 0))))

(fn SetBatteryColor
  (bind _battery_ui (Variables|Default|GetBattery%20UI))
  (Utilities|IsValid _battery_ui
    (:Is%20Valid
      (Default|SetCellColor _battery_ui (Variables|Default|GetHealth)))))