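; Game mode for RG4 that restarts the current level one second after the player's BP_RobotPawn is destroyed.
; On BeginPlay it stores the "Fun" player start location, then shares the Respawn path, which binds the pawn's destroy event and sends negative damage to its health component.
; A separate function creates the battery UI widget, though nothing in this Blueprint calls it.
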(event Custom|Respawn
  (bind _asbp_robot_pawn (Utilities|Casting|CastToBP_RobotPawn (Game|GetPlayerCharacter 0)))
  (Game|BindEventtoOnDestroyed _asbp_robot_pawn (delegate Custom|OnDestroyed_Event))
  (Default|OnTakeAnyDamage (Variables|/Game/RG4/Core/BP_RobotPawn.BP_RobotPawn_C|GetBP_HealthComponent _asbp_robot_pawn) 0 -5.0))

(event Custom|OnDestroyed_Event
  (params (DestroyedActor :type Actor%20Object%20Reference))
  (Utilities|FlowControl|Delay 1.0)
  (bind _returnvalue (Game|GetCurrentLevelName true))
  (Game|OpenLevel(byName) (Utilities|String|StringToName _returnvalue)))

(event EventBeginPlay
  (CallFunction|SetInitialSpawn)
  (bind _asbp_robot_pawn (Utilities|Casting|CastToBP_RobotPawn (Game|GetPlayerCharacter 0)))
  (Game|BindEventtoOnDestroyed _asbp_robot_pawn (delegate Custom|OnDestroyed_Event))
  (Default|OnTakeAnyDamage (Variables|/Game/RG4/Core/BP_RobotPawn.BP_RobotPawn_C|GetBP_HealthComponent _asbp_robot_pawn) 0 -5.0))

(fn ConstructionScript)

(fn SetInitialSpawn
  (params (Actor :type Actor%20Object%20Reference))
  (Variables|Default|SetSpawnTransform (Transformation|GetActorLocation (Class|GameModeBase|FindPlayerStart (Game|GetGameMode) (Game|GetPlayerController 0) "Fun"))))

(fn SetBatteryUI
  (bind _returnvalue (UserInterface|CreateWidget "/Game/RG4/Core/EnergySystem/WBP_BatteryUI.WBP_BatteryUI_C" (Game|GetPlayerController 0)))
  (UserInterface|Viewport|AddtoViewport _returnvalue 0)
  (Variables|Default|SetBatteryUI _returnvalue))