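; Player robot character with camera-relative movement, jump with mid-air montage, hold-to-sprint and two traversal abilities: dash and grapple.
; Dash launches along actor forward with gravity briefly suspended, recharging on ground or after a cooldown; the input-direction branch is bypassed.
; Grapple targets the nearest BP_GrapplePoint, switches to Flying and shows a cable; Tick applies strafe-steered pull until close or released.
; The on-screen grapple-point filter is left disconnected.
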(event EventBeginPlay
  (Variables|Default|SetDefaii;t%20Walk%20Speed (Variables|/Script/Engine.CharacterMovementComponent|GetMaxWalkSpeed (Variables|Character|GetCharacterMovement))))

(event Collision|EventActorBeginOverlap
  (params (OtherActor :type Actor%20Object%20Reference)))

(event EventTick
  (params (DeltaSeconds :type Float%20%28single-precision%29)))

(event EventTick
  (params (DeltaSeconds :type Float%20%28single-precision%29))
  ;[0 0 0] Tick Events
  ;;[0 0 0] Check for dash reset
  (if (Variables|Default|GetHasDash)
    _
    (else
      (Variables|Default|SetDash%20Cooldown (+ DeltaSeconds (Variables|Default|GetDash%20Cooldown)))
      (if (or (AI|Components|NavMovement|IsMovingonGround (Variables|Character|GetCharacterMovement)) (>= (Variables|Default|GetDash%20Cooldown) 3.0))
        (Variables|Default|SetHasDash true)
        (Development|PrintString "Dash Reset"))))
  ;;[0 0 0] Apply Grapple Force
  (if (Variables|Default|GetIsGrapple)
    (Physics|AddForce (Variables|Character|GetCharacterMovement) (* (Math|Vector|Normalize (+ (Math|Vector|GetUnitDirection(Vector) (Transformation|GetActorLocation) (Variables|Default|GetGrapple%20Point%20Location)) (* (Input|AxisValues|GetMoveRight) (Transformation|GetActorRightVector) 0.5))) 3e+05))
    (Variables|/Script/CableComponent.CableComponent|SetEndLocation (Variables|Default|GetCable) (Math|Transform|InverseTransformLocation (Transformation|GetActorTransform) (Variables|Default|GetGrapple%20Point%20Location)))
    (if (<= (Math|Vector|Distance(Vector) (Variables|Default|GetGrapple%20Point%20Location) (Transformation|GetActorLocation)) 1e+02)
      (Variables|Default|SetIsGrapple false))))

(event Input|ActionEvents|InputActionJump
  (params (Key :type Key%20Structure :default "None"))
  ;[0 0 0] Jump + Double Jump
  (:Pressed
    (if (< (Variables|Default|GetJumpCurrentCount) (Variables|Default|GetJumpMaxCount))
      (if (AI|Components|NavMovement|IsFalling (Variables|Character|GetCharacterMovement))
        (Animation|PlayAnimMontage 0 1.0 "None")
        (Character|Jump)
        (else
          (Character|Jump)))))
  (:Released
    (Character|StopJumping)))

(event Input|ActionEvents|InputActionSprint
  (params (Key :type Key%20Structure :default "None"))
  ;[0 0 0] Sprint Toggle Logic
  (:Pressed
    (Variables|/Script/Engine.CharacterMovementComponent|SetMaxWalkSpeed (Variables|Character|GetCharacterMovement) (* 3.0 (Variables|Default|GetDefaii;t%20Walk%20Speed))))
  (:Released
    (Variables|/Script/Engine.CharacterMovementComponent|SetMaxWalkSpeed (Variables|Character|GetCharacterMovement) (Variables|Default|GetDefaii;t%20Walk%20Speed))))

(event Input|ActionEvents|InputActionGrapple
  (params (Key :type Key%20Structure :default "None"))
  ;[0 0 0] Find Best GrapplePoint on press Grapple button
  (:Pressed
    (bind _outactors (Actor|GetAllActorsOfClass "/Game/RG4/Placeables/BP_GrapplePoint.BP_GrapplePoint_C"))
    (Variables|Default|SetGrapple%20Point%20Location (Transformation|GetActorLocation (.ReturnValue (Actor|FindNearestActor (Transformation|GetWorldLocation (Variables|Collision|GetCapsuleComponent)) _outactors))))
    (Variables|Default|SetIsGrapple true)
    (Pawn|Components|CharacterMovement|SetMovementMode (Variables|Character|GetCharacterMovement) "MOVE_Flying" 0)
    (Rendering|SetVisibility (Variables|Default|GetCable) true false))
  (:Released
    (Variables|Default|SetIsGrapple false)
    (Pawn|Components|CharacterMovement|SetMovementMode (Variables|Character|GetCharacterMovement) "MOVE_Falling" 0)
    (Rendering|SetVisibility (Variables|Default|GetCable) false false)))

(event Input|ActionEvents|InputActionDash
  (params (Key :type Key%20Structure :default "None"))
  (bind _camera (Variables|Default|GetCamera))
  (bind _returnvalue (Math|Vector|GetForwardVector _camera))
  (bind (_x _y) (Class|KismetMathLibrary|BreakVector3f _returnvalue))
  ;[0 0 0] Dash (Ground and Mid-air)
  (:Pressed
    (if (Variables|Default|GetHasDash)
      (Development|PrintString "Dashed")
      (Variables|Default|SetHasDash false)
      (Variables|Default|SetDash%20Cooldown 0.0)
      (Utilities|FlowControl|DoOnce false :!label _label
        (:Completed
          (Character|LaunchCharacter "0.000000,0.000000,100.000000" false false)
          (Utilities|FlowControl|Delay 0.01)
          (if true
            (Character|LaunchCharacter (* (Math|Vector|GetForwardVector (Transformation|GetActorRotation)) 1.2e+03) false false)
            (else
              (Character|LaunchCharacter (* (Math|Vector|RotateVector (Math|Vector|MakeVector (Input|AxisValues|GetMoveForward) (Input|AxisValues|GetMoveRight) 0.0) (Math|Conversions|RotationFromXVector (Math|Vector|MakeVector _x _y 0.0))) 1.2e+03) true false)))
          (Animation|PlayAnimMontage 0 1.0 "None")
          (Variables|/Script/Engine.CharacterMovementComponent|SetGravityScale (Variables|Character|GetCharacterMovement) 0.0)
          (Utilities|FlowControl|Delay 0.25)
          (Variables|/Script/Engine.CharacterMovementComponent|SetGravityScale (Variables|Character|GetCharacterMovement) 5.0)
          (goto _label Reset))))))

(event Input|AxisEvents|InputAxisMoveForward
  (params (AxisValue :type Float%20%28single-precision%29))
  (bind _returnvalue (Pawn|GetControlRotation :!class /Script/Engine.Pawn))
  (bind (_roll _pitch _yaw) (Math|Rotator|BreakRotator _returnvalue))
  ;[0 0 0 1 30] Directional Movement Logic
  (Pawn|Input|AddMovementInput (Math|Vector|GetForwardVector (Math|Rotator|MakeRotator 0.0 _pitch _yaw)) AxisValue false))

(event Input|AxisEvents|InputAxisMoveRight
  (params (AxisValue :type Float%20%28single-precision%29))
  (bind _returnvalue (Pawn|GetControlRotation :!class /Script/Engine.Pawn))
  (bind (_roll _pitch _yaw) (Math|Rotator|BreakRotator _returnvalue))
  ;[0 0 0 1 30] Directional Movement Logic
  (Pawn|Input|AddMovementInput (Math|Vector|GetRightVector (Math|Rotator|MakeRotator 0.0 _pitch _yaw)) AxisValue false))

(event Input|AxisEvents|InputAxisTurn
  (params (AxisValue :type Float%20%28single-precision%29))
  ;[0 0 0] Mouse Look Logic
  (Pawn|Input|AddControllerYawInput AxisValue))

(event Input|AxisEvents|InputAxisLookUp
  (params (AxisValue :type Float%20%28single-precision%29))
  ;[0 0 0] Mouse Look Logic
  (Pawn|Input|AddControllerPitchInput AxisValue))

(fn ConstructionScript)