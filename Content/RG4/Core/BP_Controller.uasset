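; BP_Controller is a player controller that handles pausing outside the main menu level.
; The Pause input uses a FlipFlop to alternate between opening and closing the pause menu, skipping LV_MainMenu by level name.
; Opening creates WBP_PauseMenu, blocks look and move input, shows the cursor with Game and UI input, and pauses the game.
; Closing removes the widget and reverses those settings.
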(event Input|ActionEvents|InputActionPause
  (params (Key :type Key%20Structure :default "None"))
  (:Pressed
    (bind _returnvalue (Game|GetCurrentLevelName true))
    (if (not (Utilities|Enum|Equal(Enum) _returnvalue "LV_MainMenu"))
      (Utilities|FlowControl|FlipFlop
        (:A
          (CallFunction|OpenPauseMenu))
        (:B
          (CallFunction|ClosePauseMenu))))))

(fn ConstructionScript)

(fn OpenPauseMenu
  (bind _returnvalue (UserInterface|CreateWidget "/Game/RG4/Core/Widgets/WBP_PauseMenu.WBP_PauseMenu_C" (Game|GetPlayerController 0)))
  (Variables|Default|SetPause%20Menu _returnvalue)
  (UserInterface|Viewport|AddtoViewport _returnvalue 0)
  (Input|SetIgnoreLookInput true)
  (Input|SetIgnoreMoveInput true)
  (Input|SetInputModeGameandUI (Game|GetPlayerController 0) (Variables|Default|GetPause%20Menu) "DoNotLock" false false)
  (Variables|/Script/Engine.PlayerController|SetbShowMouseCursor (Game|GetPlayerController 0) true)
  (Game|SetGamePaused true))

(fn ClosePauseMenu
  (bind _returnvalue (Game|GetPlayerController 0))
  (Widget|RemovefromParent (Variables|Default|GetPause%20Menu))
  (Input|SetInputModeGameOnly _returnvalue false)
  (Variables|/Script/Engine.PlayerController|SetbShowMouseCursor _returnvalue false)
  (Game|SetGamePaused false)
  (Input|SetIgnoreLookInput false)
  (Input|SetIgnoreMoveInput false))